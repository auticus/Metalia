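; Enemy melee attack ability that turns the avatar toward its combat target and plays a random light attack montage.
; It updates facing through enemy interface messages, then pulls the montage from the avatar's combat interface.
; The ability ends on the melee attack gameplay event or when the montage completes, is interrupted or is cancelled.
; The montage is not stopped when the ability ends, and no damage is applied here.
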(event Ability|EventActivateAbility
  (CallFunction|ProcessEnemyLogic)
  (bind _ascombat_interface (Utilities|Casting|CastToCombatInterface (Ability|GetAvatarActorfromActorInfo)))
  (|PlayMontageandWaitProxy "None" (Class|CombatInterface|GetRandomLightAttackMontage _ascombat_interface) 1.0 "" false 1.0 0.0 false
    (:then
      (Ability|Tasks|WaitGameplayEvent "(TagName=\"Event.Montage.Attack.Melee\")" 0
        (:EventReceived
          _)))
    (:OnCompleted
      _)
    (:OnInterrupted
      _)
    (:OnCancelled
      _))
  (Ability|EndAbility))

(event Ability|EventOnEndAbility
  (params (bWasCancelled :type Boolean)))

(fn ProcessEnemyLogic
  (bind _returnvalue (Ability|GetAvatarActorfromActorInfo))
  (Utilities|Casting|CastToEnemyInterface _returnvalue)
  ;[1 1 1] Get the target the enemy
  ; class is targeting
  (bind _returnvalue_2 (Class|EnemyInterface|GetCombatTarget(Message) _returnvalue))
  ;[1 1 1] BP_EnemyBase implements this
  (Class|CombatInterface|UpdateFacingTarget(Message) _returnvalue (Transformation|GetActorLocation _returnvalue_2)))