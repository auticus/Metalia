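; Melee attack gameplay ability that plays the first section of the one-handed attack montage.
; On activation, enemy avatars turn toward their combat target through interface calls, and combat avatars supply their equipped weapon to initialize the damage spec handle once.
; As the montage starts, it waits for the melee montage gameplay event and ends the ability on receipt, without applying damage in this graph.
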(event Ability|EventActivateAbility
  (CallFunction|ProcessEnemyLogic)
  (CallFunction|SetWeaponMetaData)
  (|PlayMontageandWaitProxy "None" "/Game/Animations/Metalia_Final_Animations/1HWeaponShield/Montages/AM_OneHand_Attacks.AM_OneHand_Attacks" 1.0 "Attack01" true 1.0 0.0 false
    (:then
      (Ability|Tasks|WaitGameplayEvent "(TagName=\"Event.Montage.Attack.Melee\")" 0
        (:EventReceived
          (Ability|EndAbility))))))

(event Ability|EventOnEndAbility
  (params (bWasCancelled :type Boolean)))

(fn ProcessEnemyLogic
  (bind _returnvalue (Ability|GetAvatarActorfromActorInfo))
  (Utilities|Casting|CastToEnemyInterface _returnvalue)
  ;[1 1 1] Get the target the enemy
  ; class is targeting
  (bind _returnvalue_2 (Class|EnemyInterface|GetCombatTarget(Message) _returnvalue))
  ;[1 1 1] BP_EnemyBase implements this
  (Class|CombatInterface|UpdateFacingTarget(Message) _returnvalue (Transformation|GetActorLocation _returnvalue_2)))

(fn SetWeaponMetaData
  (bind _ascombat_interface (Utilities|Casting|CastToCombatInterface (Ability|GetAvatarActorfromActorInfo)))
  (if (not (Variables|Default|GetbIsInitialized))
    (Class|MetaliaMeleeAttack|SetWeapon (Class|CombatInterface|GetEquippedWeapon _ascombat_interface))
    ;[1 1 1] This sets Is Initialized = true
    (Class|MetaliaMeleeAttack|InitializeDamageSpecHandlewithWeapon)))